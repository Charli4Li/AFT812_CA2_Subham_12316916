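; BP_Door is a door that slides upward when its associated pressure plate activates and the door's key check passes.
; On BeginPlay it binds to the plate's activated and deactivated dispatchers.
; Activation asks the plate to check for DoorKey, then plays a timeline that lerps DoorBody's relative location, or prints a message if the key is missing.
; Deactivation reverses the timeline without a key check, lowering the door.
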(event `self.ReceiveBeginPlay`
  (add `/Game/Bluprint/BP_PressurePlate.ED_PressurePlateActivated` (`self.Associated Pressure Plate`) (delegate `Door Open Signal`))
  (add `/Game/Bluprint/BP_PressurePlate.ED_PressurePlateDeactivated` (`self.Associated Pressure Plate`) (delegate `Door Close Signal`)))

(event `Door Open Signal`
  (bind _contains_key (`/Game/Bluprint/BP_PressurePlate.Check For Key` (`self.Associated Pressure Plate`) (`self.Door Key`)))
  (if _contains_key
    (bind (_direction _door_activated_track) (`Timeline|Door Actiavted` :!label _label)
      (:`Update`
        (`SceneComponent.K2_SetRelativeLocation` (`self.Door_Body`) (`KismetMathLibrary.VLerp` (0.0 0.0 0.0) (0.0 0.0 200.0) _door_activated_track) false false)))
    (else
      (`KismetSystemLibrary.PrintString` "Does not Contain Key" true true (struct :`R` 1.0 :`G` 0.85698 :`A` 1.0)))))

(event `Door Close Signal`
  (goto _label :!via `Reverse`))

(fn `UserConstructionScript`)